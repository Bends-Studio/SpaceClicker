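; CameraMan_BP is a camera pawn that moves the view between two levels: a focused NCoin view and the wider planets view.
; BeginPlay caches the starting location and rotation, which the SmoothPlanetView timeline lerps toward the planet-view transform, playing forward outward and in reverse back.
; AnimationFinished and NCoinIsNowFocused flags gate both transitions.
; Going outward also rebuilds the main interface widget and clears the game mode's NCoin shop flag.
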(event Custom|Planets%20View
  ;[0 1 0] Poruszanie się kamery pomiędzy "poziomami"
  (|CameraAnimation))

(event Custom|Going%20back%20to%20planet%20View
  ;[0 1 0] Poruszanie się kamery pomiędzy "poziomami"
  (|CameraAnimation) ; enters at Going to Planet View
)

(event EventBeginPlay
  ;[0 1 0] Przypisywanie podstawowej rotacji i lokacji
  (CallFunction|GettingStertedLocationandRotation))

(fn ConstructionScript)

(fn GettingStertedLocationandRotation
  (Variables|Default|SetStarted%20Location (Transformation|GetWorldLocation (Variables|Default|GetDefaultSceneRoot)))
  (Variables|Default|SetStarted%20Rotation (Transformation|GetWorldRotation (Variables|Default|GetCamera))))

(fn CasttoGamemode
  (bind _asgamemodebase_bp (Utilities|Casting|CastToGamemodebase_BP (Game|GetGameMode)))
  (return _asgamemodebase_bp))