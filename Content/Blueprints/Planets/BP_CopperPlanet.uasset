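; BP_CopperPlanet is a tappable planet in a clicker game that earns NCoin.
; Looping timelines spin the planet mesh and yaw an Arrow component for its motion around the sun.
; A touch adds one NCoin plus the AddingClicks bonus from MainInterface_UI and replays a scale animation.
; It also lerps the CameraMan_BP pawn toward the planet, stopping the orbit timeline when that move finishes.
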(event OnInputTouchBegin(NCoinPlanet)
  (params (FingerIndex :type ETouchIndex%20Enum :default "Touch1") (TouchedComponent :type Primitive%20Component%20Object%20Reference))
  (Utilities|FlowControl|Sequence
    (:then_0
      ;[1 1 1] Click + Adding clicks from shop
      (bind _foundwidgets (Widget|GetAllWidgetsOfClass "/Game/UI/MainInterface_UI.MainInterface_UI_C" true))
      (bind _asmain_interface_ui (Utilities|Casting|CastToMainInterface_UI (Utilities|Array|Get(acopy) _foundwidgets)))
      (Variables|Default|SetNCoin (+ (Variables|Default|GetNCoin) 1.0 (Variables|/Game/UI/MainInterface_UI.MainInterface_UI_C|GetAddingClicks _asmain_interface_ui))))
    (:then_1
      ;[1 1 1] Camera Movement
      (bind _ascamera_man_bp (Utilities|Casting|CastToCameraMan_BP (Game|Player|GetPlayerPawn 0)))
      (bind (_direction _movement _rotation) (Timeline|Smooth Play)
        (:Update
          (Transformation|SetWorldLocation (Variables|/Game/Pawn/CameraMan_BP.CameraMan_BP_C|GetDefaultSceneRoot _ascamera_man_bp) (Math|Vector|Lerp(Vector) (Transformation|GetWorldLocation (Variables|/Game/Pawn/CameraMan_BP.CameraMan_BP_C|GetDefaultSceneRoot _ascamera_man_bp)) (- (Transformation|GetWorldLocation (Variables|Default|GetNCoinPlanet)) "300.000000, 0, 0") _movement) false false)
          (Transformation|SetWorldRotation (Variables|/Game/Pawn/CameraMan_BP.CameraMan_BP_C|GetCamera _ascamera_man_bp) (Math|Rotator|Lerp(Rotator) (Transformation|GetWorldRotation (Variables|/Game/Pawn/CameraMan_BP.CameraMan_BP_C|GetCamera _ascamera_man_bp)) "0, 0, 0" _rotation) false false))
        (:Finished
          ;[1 1 1] Rotating planet
          (bind _spin (Timeline|rotation%20around%20sun Stop)
            (:Update
              (Transformation|SetWorldRotation (Variables|Default|GetArrow) (Math|Rotator|MakeRotator 0.0 0.0 _spin) false false))
            (:Finished
              (Timeline|rotation%20around%20sun PlayFromStart))))))
    (:then_2
      ;[1 1 1] Scale After Click
      (bind _newtrack_0 (Timeline|Scale%20planet PlayFromStart)
        (:Update
          (Transformation|SetWorldScale3D (Variables|Default|GetNCoinPlanet) _newtrack_0))))))

(event EventBeginPlay
  (Utilities|FlowControl|Sequence
    (:then_1
      ;[1 1 1] Spinnig
      (bind _rotationplanet (Timeline|Rotating%20Planet Play)
        (:Update
          (Transformation|SetWorldRotation (Variables|Default|GetNCoinPlanet) (Math|Rotator|MakeRotator 0.0 0.0 _rotationplanet) false false))
        (:Finished
          (Timeline|Rotating%20Planet PlayFromStart))))
    (:then_2
      ;[1 1 1] Rotating planet
      (bind _spin (Timeline|rotation%20around%20sun Play)
        (:Update
          (Transformation|SetWorldRotation (Variables|Default|GetArrow) (Math|Rotator|MakeRotator 0.0 0.0 _spin) false false))
        (:Finished
          (Timeline|rotation%20around%20sun PlayFromStart))))))

(fn ConstructionScript)