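; Clickable NCoin planet for a clicker game, orbiting and spinning on looping timelines while holding the NCoin and Fuel totals.
; Touch adds coins plus MainInterface_UI's shop bonus, pulses scale, eases CameraMan_BP to the planet, then pauses orbit and shows CameraReturn.
; GoingBackCamera restores the saved camera transform and resumes orbit.
; Timeline-and-Delay loops drive passive income from ClicksPerSecounds and fuel production, which BuyingaFuel starts for an NCoin cost.
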(event OnInputTouchBegin(NCoinPlanet)
  (params (FingerIndex :type ETouchIndex%20Enum :default "Touch1") (TouchedComponent :type Primitive%20Component%20Object%20Reference))
  (Utilities|FlowControl|Sequence
    (:then_0
      ;[1 1 1] Click + Adding clicks from shop
      (bind _foundwidgets (Widget|GetAllWidgetsOfClass "/Game/UI/MainInterface_UI.MainInterface_UI_C" true))
      (bind _asmain_interface_ui (Utilities|Casting|CastToMainInterface_UI (Utilities|Array|Get(acopy) _foundwidgets)))
      (Variables|Default|SetNCoin (+ (Variables|Default|GetNCoin) 1.0 (Variables|/Game/UI/MainInterface_UI.MainInterface_UI_C|GetAddingClicks _asmain_interface_ui))))
    (:then_1
      ;[1 1 1] Camera Movement
      (bind _ascamera_man_bp (Utilities|Casting|CastToCameraMan_BP (Game|Player|GetPlayerPawn 0)))
      (bind (_direction _movement _rotation) (Timeline|Smooth PlayFromStart)
        (:Update
          (Transformation|SetWorldLocation (Variables|/Game/Pawn/CameraMan_BP.CameraMan_BP_C|GetDefaultSceneRoot _ascamera_man_bp) (Math|Vector|Lerp(Vector) (Transformation|GetWorldLocation (Variables|/Game/Pawn/CameraMan_BP.CameraMan_BP_C|GetDefaultSceneRoot _ascamera_man_bp)) (- (Transformation|GetWorldLocation (Variables|Default|GetNCoinPlanet)) "300.000000, 0, 0") _movement) false false)
          (Transformation|SetWorldRotation (Variables|/Game/Pawn/CameraMan_BP.CameraMan_BP_C|GetCamera _ascamera_man_bp) (Math|Rotator|Lerp(Rotator) (Transformation|GetWorldRotation (Variables|/Game/Pawn/CameraMan_BP.CameraMan_BP_C|GetCamera _ascamera_man_bp)) "0, 0, 0" _rotation) false false))
        (:Finished
          (Utilities|FlowControl|Sequence
            (:then_0
              ;[1 1 1] Rotating planet
              (bind _spin (Timeline|rotation%20around%20sun Stop)
                (:Update
                  (Transformation|SetWorldRotation (Variables|Default|GetArrow) (Math|Rotator|MakeRotator 0.0 0.0 _spin) false false))
                (:Finished
                  (Timeline|rotation%20around%20sun PlayFromStart))))
            (:then_1
              (Variables|Default|SetisFocused? true)
              (bind _foundwidgets_2 (Widget|GetAllWidgetsOfClass "/Game/UI/MainInterface_UI.MainInterface_UI_C" true))
              (bind _asmain_interface_ui_2 (Utilities|Casting|CastToMainInterface_UI (Utilities|Array|Get(acopy) _foundwidgets_2)))
              (Widget|SetVisibility (Variables|/Game/UI/MainInterface_UI.MainInterface_UI_C|GetCameraReturn _asmain_interface_ui_2) "Visible"))))))
    (:then_2
      ;[1 1 1] Scale After Click
      (bind _newtrack_0 (Timeline|Scale%20planet PlayFromStart)
        (:Update
          (Transformation|SetWorldScale3D (Variables|Default|GetNCoinPlanet) _newtrack_0))))))

(event Custom|GoingBackCamera
  ;[1 1 1] Backward camera movement after Click
  (if (Variables|Default|GetisFocused?)
    (bind _ascamera_man_bp (Utilities|Casting|CastToCameraMan_BP (Game|Player|GetPlayerPawn 0)))
    (bind (_direction _movement _rotation) (Timeline|Backward%20Rotation%20and%20Location PlayFromStart)
      (:Update
        (Transformation|SetWorldLocation (Variables|/Game/Pawn/CameraMan_BP.CameraMan_BP_C|GetDefaultSceneRoot _ascamera_man_bp) (Math|Vector|Lerp(Vector) (Transformation|GetWorldLocation (Variables|/Game/Pawn/CameraMan_BP.CameraMan_BP_C|GetDefaultSceneRoot _ascamera_man_bp)) (Variables|Default|GetStartCameraLocation) _movement) false false)
        (Transformation|SetWorldRotation (Variables|/Game/Pawn/CameraMan_BP.CameraMan_BP_C|GetCamera _ascamera_man_bp) (Math|Rotator|Lerp(Rotator) (Transformation|GetWorldRotation (Variables|/Game/Pawn/CameraMan_BP.CameraMan_BP_C|GetCamera _ascamera_man_bp)) (Variables|Default|GetStartCameraRotation) _rotation) false false)
        (bind _foundwidgets (Widget|GetAllWidgetsOfClass "/Game/UI/MainInterface_UI.MainInterface_UI_C" true))
        (bind _asmain_interface_ui (Utilities|Casting|CastToMainInterface_UI (Utilities|Array|Get(acopy) _foundwidgets)))
        (Widget|SetVisibility (Variables|/Game/UI/MainInterface_UI.MainInterface_UI_C|GetCameraReturn _asmain_interface_ui) "Hidden"))
      (:Finished
        (Variables|Default|SetisFocused? false)
        (CallFunction|StartPlanetMovement)))))

(event Custom|Start%20Planet%20Movement
  ;[1 1 1] Rotating planet
  (bind _spin (Timeline|rotation%20around%20sun Play)
    (:Update
      (Transformation|SetWorldRotation (Variables|Default|GetArrow) (Math|Rotator|MakeRotator 0.0 0.0 _spin) false false))
    (:Finished
      (Timeline|rotation%20around%20sun PlayFromStart))))

(event Custom|Buying%20a%20Fuel
  ;[1 1 1] Buying fuel per secound
  (if (>= (Variables|Default|GetNCoin) 1.5e+03)
    (Variables|Default|SetNCoin (- (Variables|Default|GetNCoin) 1.5e+03))
    (Utilities|FlowControl|Delay 0.0 :!label _label)
    (bind _fuelpersecound (Timeline|FuelPerSecound Play)
      (:Update
        (Variables|Default|SetFuel (Math|Float|Lerp (Variables|Default|GetFuel) (+ (Variables|Default|GetFuel) (Variables|Default|GetFuelPerSecounds)) _fuelpersecound)))
      (:Finished
        (goto _label)))))

(event EventBeginPlay
  (Utilities|FlowControl|Sequence
    (:then_0
      ;[1 1 1] Autoclick from shop
      (Utilities|FlowControl|Delay 0.0 :!label _label)
      (bind _foundwidgets (Widget|GetAllWidgetsOfClass "/Game/UI/MainInterface_UI.MainInterface_UI_C" true))
      (bind _asmain_interface_ui (Utilities|Casting|CastToMainInterface_UI (Utilities|Array|Get(acopy) _foundwidgets)))
      (bind _smooth (Timeline|SmothNumbers Play)
        (:Update
          (Variables|Default|SetNCoin (Math|Float|Lerp (Variables|Default|GetNCoin) (+ (Variables|Default|GetNCoin) (Variables|/Game/UI/MainInterface_UI.MainInterface_UI_C|GetClicksPerSecounds _asmain_interface_ui)) _smooth)))
        (:Finished
          (goto _label))))
    (:then_1
      ;[1 1 1] Rotating planet
      (bind _spin (Timeline|rotation%20around%20sun Play)
        (:Update
          (Transformation|SetWorldRotation (Variables|Default|GetArrow) (Math|Rotator|MakeRotator 0.0 0.0 _spin) false false))
        (:Finished
          (Timeline|rotation%20around%20sun PlayFromStart))))
    (:then_2
      (bind _ascamera_man_bp (Utilities|Casting|CastToCameraMan_BP (Game|Player|GetPlayerPawn 0)))
      (Variables|Default|SetStartCameraLocation (Transformation|GetWorldLocation (Variables|/Game/Pawn/CameraMan_BP.CameraMan_BP_C|GetDefaultSceneRoot _ascamera_man_bp)))
      (Variables|Default|SetStartCameraRotation (Transformation|GetWorldRotation (Variables|/Game/Pawn/CameraMan_BP.CameraMan_BP_C|GetCamera _ascamera_man_bp))))
    (:then_3
      ;[1 1 1] Spinnig
      (bind _rotationplanet (Timeline|Rotating%20Planet Play)
        (:Update
          (Transformation|SetWorldRotation (Variables|Default|GetNCoinPlanet) (Math|Rotator|MakeRotator 0.0 0.0 _rotationplanet) false false))
        (:Finished
          (Timeline|Rotating%20Planet PlayFromStart))))))

(fn ConstructionScript)