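; Game mode for a planet-themed clicker game that holds the NCoin economy and, on start, creates the main UI and background music.
; Planet clicks add the per-click amount; house and farm purchases raise click and autoclick income, with multiplicatively growing costs.
; Buying a farm also triggers a one-time start of a self-restarting timeline that adds autoclick income smoothly using delta time.
; The shop opens only when the camera pawn has the NCoin planet focused.
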(event Custom|Click%20on%20NCPlanet
  ;[0 1 0] Zliczanie kliknięć + Kupione kliknięcia
  (CallFunction|NCoingCounter))

(event Custom|Open%20Shop
  ;[1 0.7706 0] Zmiana UI przy innej planecie
  (CallFunction|MultipleShops))

(event Custom|Buying%20House
  ;[0 1 0] Dodawanie kliknięć po zakupie domu
  (CallFunction|AddingMoreClickwhenBuyAHouse))

(event Custom|Buying%20Farm
  ;[0 1 0] Autoclick na sekundę + dowania kliknięć po zakupie Farmy
  (Utilities|FlowControl|Sequence
    (:then_0
      (CallFunction|AddingAutoclickAfterBuyAFarm))
    (:then_1
      (|Autoclick))))

(event EventBeginPlay
  ;[0 1 0] Tworzenie MainUI i Odtwarzanie muzyki
  (bind _returnvalue (UserInterface|CreateWidget "/Game/UI/UI_MainInterface.UI_MainInterface_C"))
  (UserInterface|Viewport|AddtoViewport _returnvalue 0)
  (bind _returnvalue_2 (Audio|CreateSound2D "/Game/Sounds/CUE_BackgroundSpace.CUE_BackgroundSpace" 1.0 1.0 0.0 0))
  (Audio|Components|Audio|Play _returnvalue_2 0.0))

(fn ConstructionScript)

(fn CasttoNCoinPlanet
  (bind _outactors (Actor|GetAllActorsOfClass "/Game/Blueprints/Planets/NCoinplanet_BP.NCoinPlanet_BP_C"))
  (return (Utilities|Array|Get(acopy) _outactors)))

(fn CasttoCopperPlanet
  (bind _outactors (Actor|GetAllActorsOfClass "/Game/Blueprints/Planets/BP_CopperPlanet.BP_CopperPlanet_C"))
  (return (Utilities|Array|Get(acopy) _outactors)))

(fn CasttoCameraman
  (bind _ascamera_man_bp (Utilities|Casting|CastToCameraMan_BP (Game|Player|GetPlayerPawn 0)))
  (return _ascamera_man_bp))

(fn MultipleShops
  (bind _ascamera_man_bp (CallFunction|CasttoCameraman))
  (if (Variables|/Game/Pawn/CameraMan_BP.CameraMan_BP_C|GetNCoin%20Is%20now%20Focused _ascamera_man_bp)
    (bind _returnvalue (UserInterface|CreateWidget "/Game/UI/UI_PlanetsShop.UI_PlanetsShop_C"))
    (UserInterface|Viewport|AddtoViewport _returnvalue 0)
    (elif true
      _)))

(fn AddingMoreClickwhenBuyAHouse
  (if (>= (Variables|Default|GetNCoin) (Variables|Default|GetNCoin%20House%20Cost))
    (Variables|Default|SetNCoin (- (Variables|Default|GetNCoin) (Variables|Default|GetNCoin%20House%20Cost)))
    (Variables|Default|SetNCoin%20per%20Click%20added (+ (Variables|Default|GetNCoin%20per%20Click%20added) 1.0))
    (Variables|Default|SetNCoin%20House%20Cost (* (Variables|Default|GetNCoin%20House%20Cost) 1.2))
    (else
      (Development|PrintString "NIE STAĆ CIĘ !"))))

(fn AddingAutoclickAfterBuyAFarm
  (if (>= (Variables|Default|GetNCoin) (Variables|Default|GetNCoin%20Farm%20Cost))
    (Variables|Default|SetNCoin (- (Variables|Default|GetNCoin) (Variables|Default|GetNCoin%20Farm%20Cost)))
    (Variables|Default|SetNCoin%20Autoclick%20Amount (+ (Variables|Default|GetNCoin%20Autoclick%20Amount) 0.25))
    (Variables|Default|SetNCoin%20Farm%20Cost (* (Variables|Default|GetNCoin%20Farm%20Cost) 1.5))
    (else
      (Development|PrintString "NIE STAĆ CIĘ !"))))

(fn NCoingCounter
  (Variables|Default|SetNCoin (+ (Variables|Default|GetNCoin) (Variables|Default|GetNCoin%20per%20Click%20added))))